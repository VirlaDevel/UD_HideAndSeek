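; Start button for a timed VR mini-game, triggered when the VR pawn overlaps it.
; It tells the BP_Goal cached at BeginPlay to spawn the first mobile, then runs a Delay-loop timer macro that updates CurrentTime by reference.
; Tick plays a ticking-clock cue within two fixed time windows.
; On timeout it plays a final sound, makes the pawn drop the mobile, destroys it and clears GameRunning.
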(event OnComponentBeginOverlap(myStarterButton)
  (params (OverlappedComponent :type Primitive%20Component%20Object%20Reference) (OtherActor :type Actor%20Object%20Reference) (OtherComp :type Primitive%20Component%20Object%20Reference) (OtherBodyIndex :type Integer) (bFromSweep :type Boolean) (SweepResult :type Hit%20Result%20Structure%20%28by%20ref%29))
  (if (== (Utilities|GetClass OtherActor) "/Game/Assets/player/bp_MyVRPawn.bp_MyVRPawn_C")
    (Audio|PlaySound2D "/Game/Assets/audio_cues/startCue.startCue")
    (Utilities|FlowControl|Sequence
      (:then_0
        (Variables|Default|SetgameRunning true)
        (Default|SpawnFirstMobile (Variables|Default|GetGoalPoste))
        (bind _outactors (Actor|GetAllActorsOfClass "/Game/Assets/blueprints/BP_myMobile.BP_myMobile_C"))
        (bind _asbp_my_mobile (Utilities|Casting|CastToBP_myMobile (Utilities|Array|Get(acopy) _outactors)))
        (Variables|Default|SetMobileRef _asbp_my_mobile))
      (:then_1
        (Utilities|Timer (Variables|Default|GetCurrentTime) (Variables|Default|GetMaxTime)
          (:Finished
            (Audio|PlaySound2D "/Game/Assets/audio_cues/finalSoundCue.finalSoundCue")
            (Default|DropObject (Variables|Default|GetmyVRPawnRef) (Variables|/Game/Assets/blueprints/BP_myMobile.BP_myMobile_C|GetAttachedMotionContr (Variables|Default|GetMobileRef)))
            (Actor|DestroyActor (Variables|Default|GetMobileRef))
            (Variables|Default|SetgameRunning false)))))))

(event EventBeginPlay
  (bind _asbp_my_vrpawn (Utilities|Casting|CastTobp_MyVRPawn (Game|Player|GetPlayerPawn 0)))
  (Variables|Default|SetmyVRPawnRef _asbp_my_vrpawn)
  (bind _outactors (Actor|GetAllActorsOfClass "/Game/Assets/blueprints/BP_Goal.BP_Goal_C"))
  (bind _asbp_goal (Utilities|Casting|CastToBP_Goal (Utilities|Array|Get(acopy) _outactors)))
  (Variables|Default|SetGoalPoste _asbp_goal))

(event Collision|EventActorBeginOverlap
  (params (OtherActor :type Actor%20Object%20Reference)))

(event EventTick
  (params (DeltaSeconds :type Float%20%28single-precision%29))
  (if (or (Math|Float|InRange(Float) (Variables|Default|GetCurrentTime) 103.0 104.0) (Math|Float|InRange(Float) (Variables|Default|GetCurrentTime) 111.0 112.0))
    (Audio|PlaySound2D "/Game/Assets/audio_cues/tickingClockCue.tickingClockCue")))

(fn ConstructionScript)