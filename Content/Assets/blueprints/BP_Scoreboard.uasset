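; BP_Scoreboard is a scoreboard actor that stays hidden until the game is running.
; On BeginPlay it hides its Cube component and children, then caches the first BP_starterButton found in the level.
; Tick polls that button's GameRunning flag and unhides the Cube hierarchy while it is true, with no path to hide it again.
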(event EventBeginPlay
  ;[1 1 1] create reference to starter button -  set invisible (cube)
  (Development|SetHiddeninGame (Variables|Default|GetCube) true true)
  (bind _outactors (Actor|GetAllActorsOfClass "/Game/Assets/blueprints/BP_starterButton.BP_starterButton_C"))
  (bind _asbp_starter_button (Utilities|Casting|CastToBP_starterButton (Utilities|Array|Get(acopy) _outactors)))
  (Variables|Default|SetstarterButton _asbp_starter_button))

(event EventTick
  (params (DeltaSeconds :type Float%20%28single-precision%29))
  ;[1 1 1] toggle visibility due to running game
  (if (Variables|/Game/Assets/blueprints/BP_starterButton.BP_starterButton_C|GetgameRunning (Variables|Default|GetstarterButton))
    (Development|SetHiddeninGame (Variables|Default|GetCube) false true)))

(fn ConstructionScript)