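; Mobile phone actor that buzzes in the world until picked up, and can be grabbed by a motion controller.
; After a short initial delay, it plays a buzz at the phone's location, repeating at random intervals through a Delay-based timer macro.
; PickUp disables physics and collision and attaches the root to the controller; DropOff reverses this.
; The buzz loop ends once it finds the phone picked, and DropOff does not restart it.
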(event EventBeginPlay
  (Utilities|FlowControl|Delay 3.0)
  (if (not (Variables|Default|GetisPicked)) :!label _label
    (Audio|PlaySoundatLocation "/Game/Assets/audio_cues/mobileBuzzCue.mobileBuzzCue" (Transformation|GetWorldLocation (Variables|Default|GetmyMobilePhone)))
    (Utilities|Timer (Variables|Default|GetCurrentTime) (Math|Random|RandomFloatinRange 8.0 16.0)
      (:Finished
        (goto _label)))))

(event Collision|EventActorBeginOverlap
  (params (OtherActor :type Actor%20Object%20Reference)))

(event EventPickUp
  (params (ActorToAttachTo :type Scene%20Component%20Object%20Reference))
  (Variables|Default|SetAttachedMotionContr ActorToAttachTo)
  (Physics|SetSimulatePhysics (Variables|Default|GetmyMobilePhone) false)
  (bind _returnvalue (Transformation|AttachComponentToComponent (VehicleSound|GetRootComponent) ActorToAttachTo "None" "KeepWorld" "KeepWorld" "KeepWorld" true))
  (Variables|Default|SetisPicked _returnvalue)
  (Collision|SetCollisionEnabled (Variables|Default|GetmyMobilePhone) "NoCollision"))

(event EventDropOff
  (Physics|SetSimulatePhysics (Variables|Default|GetmyMobilePhone) true)
  (Transformation|DetachFromActor "KeepWorld" "KeepWorld" "KeepWorld")
  (Variables|Default|SetAttachedMotionContr 0)
  (Variables|Default|SetisPicked false)
  (Collision|SetCollisionEnabled (Variables|Default|GetmyMobilePhone) "QueryAndPhysics"))

(event EventTick
  (params (DeltaSeconds :type Float%20%28single-precision%29)))

(fn ConstructionScript)