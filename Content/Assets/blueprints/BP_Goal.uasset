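; BP_Goal is the goal in a VR seek game, scoring points when the player brings a mobile device into its trigger box.
; While the starter button's game is running, an overlapping held mobile adds to the score, is dropped from the pawn's hand and destroyed, and a replacement spawns.
; Mobiles spawn at shuffled BP_mobileSpawn points, removed as used and refilled when empty, and the first-spawn event resets the score.
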(event OnComponentBeginOverlap(triggerbox)
  (params (OverlappedComponent :type Primitive%20Component%20Object%20Reference) (OtherActor :type Actor%20Object%20Reference) (OtherComp :type Primitive%20Component%20Object%20Reference) (OtherBodyIndex :type Integer) (bFromSweep :type Boolean) (SweepResult :type Hit%20Result%20Structure%20%28by%20ref%29))
  ;[1 1 1] Counting points if mobile device is placed in goal - respawn mobile
  (bind _asbp_my_mobile (Utilities|Casting|CastToBP_myMobile OtherActor))
  (if (Math|Boolean|ANDBoolean (Variables|/Game/Assets/blueprints/BP_myMobile.BP_myMobile_C|GetisPicked _asbp_my_mobile) (== (Utilities|GetClass OtherActor) "/Game/Assets/blueprints/BP_myMobile.BP_myMobile_C") (Variables|/Game/Assets/blueprints/BP_starterButton.BP_starterButton_C|GetgameRunning (Variables|Default|GetstarterButton)))
    (Variables|Default|SetScore (+ (Variables|Default|GetScore) (Variables|Default|GetScoringPoint)))
    (Default|DropObject (Variables|Default|GetmyVRPawnRef) (Variables|/Game/Assets/blueprints/BP_myMobile.BP_myMobile_C|GetAttachedMotionContr _asbp_my_mobile))
    (Actor|DestroyActor _asbp_my_mobile)
    (CallFunction|SpawnNewMobile)))

(event Custom|spawnNewMobile
  ;[1 1 1] Counting points if mobile device is placed in goal - respawn mobile
  (if (> (Utilities|Array|Length (Variables|Default|GetPossivleSpawns)) 0)
    _
    (else
      (bind _outactors (Actor|GetAllActorsOfClass "/Game/Assets/blueprints/BP_mobileSpawn.BP_mobileSpawn_C"))
      (Utilities|Array|Shuffle _outactors)
      (Variables|Default|SetPossivleSpawns _outactors)))
  (Game|SpawnActorfromClass "/Game/Assets/blueprints/BP_myMobile.BP_myMobile_C" (Transformation|GetActorTransform (Utilities|Array|Get(acopy) (Variables|Default|GetPossivleSpawns))) "Undefined" 0 0)
  (Utilities|Array|RemoveIndex (Variables|Default|GetPossivleSpawns)))

(event Custom|spawnFirstMobile
  ;[1 1 1] Event to spawn first mobile device
  (Variables|Default|SetScore 0)
  (Game|SpawnActorfromClass "/Game/Assets/blueprints/BP_myMobile.BP_myMobile_C" (Transformation|GetActorTransform (Utilities|Array|Get(acopy) (Variables|Default|GetPossivleSpawns))) "Undefined" 0 0)
  (Utilities|Array|RemoveIndex (Variables|Default|GetPossivleSpawns)))

(event EventBeginPlay
  ;[1 1 1] Get possible spawns for mobile and spawn first object to seek
  (bind _asbp_my_vrpawn (Utilities|Casting|CastTobp_MyVRPawn (Game|Player|GetPlayerPawn 0)))
  (Variables|Default|SetmyVRPawnRef _asbp_my_vrpawn)
  (bind _outactors (Actor|GetAllActorsOfClass "/Game/Assets/blueprints/BP_mobileSpawn.BP_mobileSpawn_C"))
  (Utilities|Array|Shuffle _outactors)
  (Variables|Default|SetPossivleSpawns _outactors)
  (bind _outactors_2 (Actor|GetAllActorsOfClass "/Game/Assets/blueprints/BP_starterButton.BP_starterButton_C"))
  (bind _asbp_starter_button (Utilities|Casting|CastToBP_starterButton (Utilities|Array|Get(acopy) _outactors_2)))
  (Variables|Default|SetstarterButton _asbp_starter_button))

(fn ConstructionScript)